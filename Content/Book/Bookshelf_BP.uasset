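; Bookshelf Blueprint that acts as a hinged door, paired with a book pile that tilts as it opens.
; The Open/CloseDoor event alternates between opening and closing through a FlipFlop, behind a DoOnce that resets when each timeline finishes.
; Opening lerps book pitch and shelf yaw from timeline tracks.
; Closing plays a separate timeline in reverse and rotates only the shelf.
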(event Custom|Open/Close%20Door
  (Utilities|FlowControl|DoOnce false :!label _label
    (:Completed
      (Utilities|FlowControl|FlipFlop
        (:A
          ;[1 1 1] Open Door
          (bind (_direction _booktrack _doortrack) (Timeline|OpenTrack PlayFromStart)
            (:Update
              (Transformation|SetRelativeRotation (Variables|Default|GetSM_BookPile) (Math|Rotator|MakeRotator 9e+01 (Math|Float|Lerp (Variables|Default|GetBookIn) (Variables|Default|GetBookOut) _booktrack) 9e+01) false false)
              (Transformation|SetRelativeRotation (Variables|Default|GetSM_Bookshelf_Single) (Math|Rotator|MakeRotator 0.0 0.0 (Math|Float|Lerp (Variables|Default|GetDoorClose) (Variables|Default|GetDoorOpen) _doortrack)) false false))
            (:Finished
              (goto _label Reset))))
        (:B
          ;[1 1 1] closedoor
          (bind _doortrack_2 (Timeline|Timeline ReverseFromEnd)
            (:Update
              (Transformation|SetRelativeRotation (Variables|Default|GetSM_Bookshelf_Single) (Math|Rotator|MakeRotator 0.0 0.0 (Math|Float|Lerp (Variables|Default|GetDoorClose) (Variables|Default|GetDoorOpen) _doortrack_2)) false false))
            (:Finished
              (goto _label Reset))))))))

(fn ConstructionScript)