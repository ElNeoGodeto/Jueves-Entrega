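; BP_LockedDoor is a door that the first-person character can open and close only while holding a key.
; A Box overlap enables input and opens a gate, and leaving disables both.
; The Door input checks HasKey, playing a locked sound without it.
; With the key, a FlipFlop plays or reverses a timeline that lerps mesh yaw between closed and open angles, and an opening sound plays at world origin.
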(event OnComponentBeginOverlap(Box)
  (params (OverlappedComponent :type Primitive%20Component%20Object%20Reference) (OtherActor :type Actor%20Object%20Reference) (OtherComp :type Primitive%20Component%20Object%20Reference) (OtherBodyIndex :type Integer) (bFromSweep :type Boolean) (SweepResult :type Hit%20Result%20Structure%20%28by%20ref%29))
  ;[1 1 1] Open Door
  (bind _asbp_first_person_character (Utilities|Casting|CastToBP_FirstPersonCharacter OtherActor))
  (Input|EnableInput (Game|GetPlayerController 0))
  ;[1 1 1] Animation
  (Utilities|FlowControl|Gate true) ; enters at Open
)

(event OnComponentEndOverlap(Box)
  (params (OverlappedComponent :type Primitive%20Component%20Object%20Reference) (OtherActor :type Actor%20Object%20Reference) (OtherComp :type Primitive%20Component%20Object%20Reference) (OtherBodyIndex :type Integer))
  ;[1 1 1] Open Door
  (Utilities|Casting|CastToBP_FirstPersonCharacter OtherActor)
  (Input|DisableInput (Game|GetPlayerController 0))
  ;[1 1 1] Animation
  (Utilities|FlowControl|Gate true) ; enters at Close
)

(event Input|ActionEvents|InputActionDoor
  (params (Key :type Key%20Structure :default "None"))
  ;[1 1 1] Open Door
  (:Pressed
    (if (Variables|/Game/FirstPerson/Blueprints/BP_FirstPersonCharacter.BP_FirstPersonCharacter_C|GetHasKey? (stale OnComponentBeginOverlap(Box) _asbp_first_person_character))
      (Audio|PlaySoundatLocation "/Game/Door/431117__inspectorj__door-front-opening-a.431117__inspectorj__door-front-opening-a" "0, 0, 0" "0, 0, 0" 1.0 1.0 0.0 0 0 0 0)
      ;[1 1 1] Animation
      (Utilities|FlowControl|Gate true
        (:Exit
          (Utilities|FlowControl|FlipFlop
            (:A
              (bind _door_track (Timeline|Open/Close%20Door Play)
                (:Update
                  (Transformation|SetRelativeRotation (Variables|Default|GetStaticMesh) (Math|Rotator|MakeRotator 0.0 0.0 (Math|Float|Lerp (Variables|Default|GetClosed%20Angle) (Variables|Default|GetOpen%20Angle) _door_track)) false false))))
            (:B
              (Timeline|Open/Close%20Door Reverse)))))
      (else
        (Audio|PlaySoundatLocation "/Game/Door/321087__benjaminnelan__door-locked.321087__benjaminnelan__door-locked" (Transformation|GetActorLocation) "0, 0, 0" 1.0 1.0 0.0 0 0 0 0)))))

(fn ConstructionScript)